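; BP_Crates is a movable crates prop that slides vertically between a closed and an open position.
; On BeginPlay it stores its placed location as open, then snaps to the closed position, offset along Z by Distance.
; The Open event plays the Move timeline, which lerps the actor to the open position without sweep, and Close reverses the same timeline.
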(event Custom|Open
  ;[1 1 1] Crates behaviour
  (bind _progress (Timeline|Move Play)
    (:Update
      (Transformation|SetActorLocation (Math|Vector|Lerp(Vector) (Variables|Behaviour|GetClosedPosition) (Variables|Behaviour|GetOpenPosition) _progress) false false))))

(event Custom|Close
  ;[1 1 1] Crates behaviour
  (bind _progress (Timeline|Move Reverse)
    (:Update
      (Transformation|SetActorLocation (Math|Vector|Lerp(Vector) (Variables|Behaviour|GetClosedPosition) (Variables|Behaviour|GetOpenPosition) _progress) false false))))

(event EventBeginPlay
  ;[1 1 1] Crates behaviour
  (bind _output_get (Variables|Behaviour|SetOpenPosition (Transformation|GetActorLocation)))
  (bind _output_get_2 (Variables|Behaviour|SetClosedPosition (Math|Vector|MakeVector (.x _output_get) (.y _output_get) (+ (.z _output_get) (Variables|Behaviour|GetDistance)))))
  (Transformation|SetActorLocation _output_get_2 false false))

(fn ConstructionScript)