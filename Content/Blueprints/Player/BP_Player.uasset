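; BP_Player is the player character, with axis-driven movement, controller look, jumping and two item slots, left and right.
; Each slot's input calls Use on its held item, passing the player.
; If the slot is empty, it line-traces from the camera along control rotation within pickup range and stores any BP_BasicItem hit.
; The Damage event only prints a debug string.
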(event EventDamage
  (Development|PrintString "Oof"))

(event Input|ActionEvents|InputActionJump
  (params (Key :type Key%20Structure :default "None"))
  ;[1 1 1] Player movement
  (:Pressed
    (Character|Jump))
  (:Released
    (Character|StopJumping)))

(event Input|ActionEvents|InputActionUseLeftItem
  (params (Key :type Key%20Structure :default "None"))
  ;[1 1 1] Using items
  (:Pressed
    (bind _leftitem (Variables|Items|GetLeftItem)
      (:then
        (Default|Use _leftitem self))
      (:else
        (bind _asbp_basic_item (Utilities|Casting|CastToBP_BasicItem (.hitactor (.HitResult (CallFunction|LineTrace (Variables|Default|GetCamera) (Pawn|GetControlRotation :!class /Script/Engine.Pawn) (Variables|Items|GetPickupRange))))))
        (Variables|Items|SetLeftItem _asbp_basic_item)))))

(event Input|ActionEvents|InputActionUseRightItem
  (params (Key :type Key%20Structure :default "None"))
  ;[1 1 1] Using items
  (:Pressed
    (bind _rightitem (Variables|Items|GetRightItem)
      (:then
        (Default|Use _rightitem self))
      (:else
        (bind _asbp_basic_item (Utilities|Casting|CastToBP_BasicItem (.hitactor (.HitResult (CallFunction|LineTrace (Variables|Default|GetCamera) (Pawn|GetControlRotation :!class /Script/Engine.Pawn) (Variables|Items|GetPickupRange))))))
        (Variables|Items|SetRightItem _asbp_basic_item)))))

(event Input|AxisEvents|InputAxisMoveForward
  (params (AxisValue :type Float%20%28single-precision%29))
  ;[1 1 1] Player movement
  (Pawn|Input|AddMovementInput (Transformation|GetActorForwardVector) AxisValue false))

(event Input|AxisEvents|InputAxisMoveRight
  (params (AxisValue :type Float%20%28single-precision%29))
  ;[1 1 1] Player movement
  (Pawn|Input|AddMovementInput (Transformation|GetActorRightVector) AxisValue false))

(event Input|AxisEvents|InputAxisTurn
  (params (AxisValue :type Float%20%28single-precision%29))
  ;[1 1 1] Camera movement
  (Pawn|Input|AddControllerYawInput AxisValue))

(event Input|AxisEvents|InputAxisLookUp
  (params (AxisValue :type Float%20%28single-precision%29))
  ;[1 1 1] Camera movement
  (Pawn|Input|AddControllerPitchInput AxisValue))

(fn ConstructionScript)