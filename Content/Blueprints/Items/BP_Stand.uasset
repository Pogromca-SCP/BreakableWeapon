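; BP_Stand is an item stand that keeps spawning sword or shield pickups throughout play.
; From BeginPlay, it waits a random delay, then randomly spawns a scaled-down BP_Sword or BP_Shield at that item's offset from the stand and plays a spawn sound there.
; A custom event re-enters the delay after each spawn, looping indefinitely without checking whether earlier items remain.
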(event Custom|F**kGoBack
  (bind _spawnsound (Variables|Sounds|GetSpawnSound))
  ;[1 1 1] Item spawning
  (Utilities|FlowControl|Delay (Math|Random|RandomFloatinRange 1e+01 25.0))
  (if (Math|Random|RandomBool)
    (bind _returnvalue (Game|SpawnActorfromClass "/Game/Blueprints/Items/BP_Sword.BP_Sword_C" (Math|Transform|MakeTransform (+ (Transformation|GetActorLocation) (Variables|Gameplay|GetWeaponSpawn)) (Variables|Gameplay|GetWeaponRot) "0.200000,0.200000,0.200000") "Undefined" 0 0))
    (Audio|PlaySoundatLocation _spawnsound (Transformation|GetActorLocation _returnvalue) "0, 0, 0" 1.0 1.0 0.0 0 0 0)
    (else
      (bind _returnvalue_2 (Game|SpawnActorfromClass "/Game/Blueprints/Items/BP_Shield.BP_Shield_C" (Math|Transform|MakeTransform (+ (Transformation|GetActorLocation) (Variables|Gameplay|GetShieldSpawn)) (Variables|Gameplay|GetShieldRot) "0.200000,0.200000,0.200000") "Undefined" 0 0))
      (Audio|PlaySoundatLocation _spawnsound (Transformation|GetActorLocation _returnvalue_2) "0, 0, 0" 1.0 1.0 0.0 0 0 0)))
  (CallFunction|F**kGoBack))

(event EventBeginPlay
  (bind _spawnsound (Variables|Sounds|GetSpawnSound))
  ;[1 1 1] Item spawning
  (Utilities|FlowControl|Delay (Math|Random|RandomFloatinRange 1e+01 25.0))
  (if (Math|Random|RandomBool)
    (bind _returnvalue (Game|SpawnActorfromClass "/Game/Blueprints/Items/BP_Sword.BP_Sword_C" (Math|Transform|MakeTransform (+ (Transformation|GetActorLocation) (Variables|Gameplay|GetWeaponSpawn)) (Variables|Gameplay|GetWeaponRot) "0.200000,0.200000,0.200000") "Undefined" 0 0))
    (Audio|PlaySoundatLocation _spawnsound (Transformation|GetActorLocation _returnvalue) "0, 0, 0" 1.0 1.0 0.0 0 0 0)
    (else
      (bind _returnvalue_2 (Game|SpawnActorfromClass "/Game/Blueprints/Items/BP_Shield.BP_Shield_C" (Math|Transform|MakeTransform (+ (Transformation|GetActorLocation) (Variables|Gameplay|GetShieldSpawn)) (Variables|Gameplay|GetShieldRot) "0.200000,0.200000,0.200000") "Undefined" 0 0))
      (Audio|PlaySoundatLocation _spawnsound (Transformation|GetActorLocation _returnvalue_2) "0, 0, 0" 1.0 1.0 0.0 0 0 0)))
  (CallFunction|F**kGoBack))

(fn ConstructionScript)