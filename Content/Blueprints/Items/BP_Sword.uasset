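; BP_Sword is a sword item that damages what its owner is aiming at and is used up after one use.
; Use line-traces from the owner's camera along the control rotation, sends DamageMessage to the hit actor, then destroys the sword.
; Update turns off physics and collision on the static mesh and sets a fixed relative offset, rotation and small scale.
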(event EventUse
  (params (Owner :type BP%20Player%20Object%20Reference))
  ;[1 1 1] Using the sword
  (Class|BPIDamageable|Damage(Message) (.hitactor (.HitResult (CallFunction|LineTrace (Variables|/Game/Blueprints/Player/BP_Player.BP_Player_C|GetCamera Owner) (Pawn|GetControlRotation Owner :!class /Script/Engine.Pawn) (Variables|Stats|GetRange)))))
  (Actor|DestroyActor))

(event EventUpdate
  (Physics|SetSimulatePhysics (Variables|Default|GetStaticMesh) false)
  (Collision|SetCollisionEnabled (Variables|Default|GetStaticMesh) "NoCollision")
  (Transformation|SetActorRelativeLocation "10.000000,10.000000,40.000000")
  (Transformation|SetActorRelativeRotation "60.000000, 0, 0")
  (Transformation|SetActorScale3D "0.100000,0.100000,0.100000"))

(fn ConstructionScript
  (|CallParentFunction))