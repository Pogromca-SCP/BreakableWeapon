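; BP_BasicItem is an item actor that can be held in either hand, with empty Use and StopUsing events.
; Pickup disables mesh physics, collision and shadows, then applies the held relative transform without attaching the actor itself.
; For the left side it mirrors the held position and offset on Y, which Drop flips back while detaching and restoring the mesh.
; DestroyItem plays a sound and particle effect before removing the actor.
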(event Custom|StopUsing
  (params (Owner :type BP%20Player%20Object%20Reference)))

(event Custom|Use
  (params (Owner :type BP%20Player%20Object%20Reference)))

(event Custom|Drop
  (params (IsLeft :type Boolean))
  ;[1 1 1] Droping the item
  (Collision|SetCollisionEnabled (Variables|Default|GetMesh) "QueryAndPhysics")
  (Physics|SetSimulatePhysics (Variables|Default|GetMesh) true)
  (Rendering|SetCastShadow (Variables|Default|GetMesh) true)
  (Transformation|DetachFromActor "KeepWorld" "KeepWorld" "KeepWorld")
  (if IsLeft
    (Variables|Gameplay|SetHoldedPosition (Math|Vector|MakeVector (.x (Variables|Gameplay|GetHoldedPosition)) (* -1 (.y (Variables|Gameplay|GetHoldedPosition))) (.z (Variables|Gameplay|GetHoldedPosition))))
    (Variables|Gameplay|SetOffset (Math|Vector|MakeVector (.x (Variables|Gameplay|GetOffset)) (* -1 (.y (Variables|Gameplay|GetOffset))) (.z (Variables|Gameplay|GetOffset))))))

(event Custom|Pickup
  (params (IsLeft :type Boolean))
  ;[1 1 1] Picking up the item
  (Physics|SetSimulatePhysics (Variables|Default|GetMesh) false)
  (Collision|SetCollisionEnabled (Variables|Default|GetMesh) "NoCollision")
  (Rendering|SetCastShadow (Variables|Default|GetMesh) false)
  (if IsLeft
    (Variables|Gameplay|SetHoldedPosition (Math|Vector|MakeVector (.x (Variables|Gameplay|GetHoldedPosition)) (* -1 (.y (Variables|Gameplay|GetHoldedPosition))) (.z (Variables|Gameplay|GetHoldedPosition))))
    (Variables|Gameplay|SetOffset (Math|Vector|MakeVector (.x (Variables|Gameplay|GetOffset)) (* -1 (.y (Variables|Gameplay|GetOffset))) (.z (Variables|Gameplay|GetOffset)))))
  (Transformation|SetActorRelativeLocation (Variables|Gameplay|GetHoldedPosition))
  (Transformation|SetActorRelativeRotation (Variables|Gameplay|GetHoldedRotation)))

(event Custom|DestroyItem
  ;[1 1 1] Destroying the item
  (Audio|PlaySoundatLocation (Variables|Sounds|GetDestructionSound) (Transformation|GetActorLocation) "0, 0, 0" 1.0 1.0 0.0 0 0 0)
  (Effects|SpawnEmitteratLocation (Variables|Particles|GetDestructionParticles) (Transformation|GetActorLocation) (Transformation|GetActorRotation))
  (Actor|DestroyActor))

(fn ConstructionScript)