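; BP_Rock is a throwable item that damages what it hits.
; On Use, it drops itself, launches its mesh along the owner's control rotation with an impulse scaled by Power, then binds the mesh's hit event.
; On a hit, it sends DamageMessage to the other actor and destroys the item.
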(event Custom|Hit
  (params (HitComponent :type Primitive%20Component%20Object%20Reference) (OtherActor :type Actor%20Object%20Reference) (OtherComp :type Primitive%20Component%20Object%20Reference) (NormalImpulse :type Vector) (Hit :type Hit%20Result%20Structure%20%28by%20ref%29))
  ;[1 1 1] Throwing the rock
  (Class|BPIDamageable|Damage(Message) OtherActor)
  (CallFunction|DestroyItem))

(event EventUse
  (params (Owner :type BP%20Player%20Object%20Reference))
  ;[1 1 1] Throwing the rock
  (CallFunction|Drop false)
  (Physics|AddImpulse (Variables|Character|GetMesh) (* (Math|Vector|GetForwardVector (Pawn|GetControlRotation Owner :!class /Script/Engine.Pawn)) (Variables|Gameplay|GetPower)) "None" false)
  (Collision|BindEventtoOnComponentHit (Variables|Character|GetMesh) (delegate Custom|Hit)))

(fn ConstructionScript
  (|CallParentFunction))